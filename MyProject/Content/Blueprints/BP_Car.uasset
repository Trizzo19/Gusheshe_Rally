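; BP_Car is a drivable vehicle Blueprint with a mouse-controlled camera and speed-based smoke effects.
; Throttle, brake, steering and handbrake inputs feed straight into the vehicle movement component, while mouse axes rotate the spring arm's pitch and yaw.
; Two smoke effects start off, and each A or D key press switches them on or off by checking absolute forward speed against a threshold.
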(event `InputAxisKey|MouseY`
  (params (AxisValue :type "Float (single-precision)"))
  ;[1 1 1] Camera
  (`SceneComponent.K2_AddRelativeRotation` (`self.SpringArm`) (`KismetMathLibrary.MakeRotator` 0.0 AxisValue) false false))

(event `InputAxisKey|MouseX`
  (params (AxisValue :type "Float (single-precision)"))
  ;[1 1 1] Camera
  (`SceneComponent.K2_AddRelativeRotation` (`self.SpringArm`) (`KismetMathLibrary.MakeRotator` 0.0 0.0 AxisValue) false false))

(event `Key|A`
  (params (Key :type "Key Structure"))
  ;[1 1 1] SmokeVFX
  (:`Pressed`
    (if (>= (`KismetMathLibrary.Abs` (`ChaosVehicleMovementComponent.GetForwardSpeed` (`self.VehicleMovementComponent`))) 800.0) :!label _label
      (`ActorComponent.SetActive` (`self.Smoke`) true false)
      (`ActorComponent.SetActive` (`self.Smoke1`) true false)
      (else
        (`ActorComponent.SetActive` (`self.Smoke1`) false false :!label _label_2)
        (`ActorComponent.SetActive` (`self.Smoke`) false false)))))

(event `InputAxis|Throttle`
  (params (AxisValue :type "Float (single-precision)"))
  ;[1 1 1] CarMovement
  (`ChaosVehicleMovementComponent.SetThrottleInput` (`self.VehicleMovementComponent`) AxisValue))

(event `Key|D`
  (params (Key :type "Key Structure"))
  ;[1 1 1] SmokeVFX
  (:`Pressed`
    (goto _label)))

(event `InputAxis|Brake`
  (params (AxisValue :type "Float (single-precision)"))
  ;[1 1 1] CarMovement
  (`ChaosVehicleMovementComponent.SetBrakeInput` (`self.VehicleMovementComponent`) AxisValue))

(event `InputAxis|Steering`
  (params (AxisValue :type "Float (single-precision)"))
  ;[1 1 1] CarMovement
  (`ChaosVehicleMovementComponent.SetSteeringInput` (`self.VehicleMovementComponent`) AxisValue))

(event `self.ReceiveBeginPlay`
  ;[1 1 1] SmokeVFX
  (goto _label_2))

(event `InputAction|Handbrake`
  (params (Key :type "Key Structure"))
  (bind _vehiclemovementcomponent (`self.VehicleMovementComponent`))
  ;[1 1 1] CarMovement
  (:`Pressed`
    (`ChaosVehicleMovementComponent.SetHandbrakeInput` _vehiclemovementcomponent true))
  (:`Released`
    (`ChaosVehicleMovementComponent.SetHandbrakeInput` _vehiclemovementcomponent false)))

(fn `UserConstructionScript`)